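; BP_LightEmotes is a spotlight Blueprint that tints its light to match an emotion: Anxiety, Sad, Worry or Anger.
; On BeginPlay it switches on CurrentEmotion and calls that emotion's event, which sets Spotlight0's color and a shared intensity.
; Each branch then calls Flickering, which applies the M_Flickering light function material when IsFlickering is true.
; The emotion is evaluated only at BeginPlay in this graph.
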(event Custom|AnxietyLight
  (bind _spotlight_0 (Variables|Default|GetSpotlight_0))
  (Rendering|Components|Light|SetLightColor _spotlight_0 (Variables|Lighting|GetAnxietyColor) true)
  (Rendering|Components|Light|SetIntensity _spotlight_0 (Variables|Lighting|GetLight%20Intensity)))

(event Custom|AngerLight
  (bind _spotlight_0 (Variables|Default|GetSpotlight_0))
  (Rendering|Components|Light|SetLightColor _spotlight_0 (Variables|Lighting|GetAngryColor) true)
  (Rendering|Components|Light|SetIntensity _spotlight_0 (Variables|Lighting|GetLight%20Intensity)))

(event Custom|WorriedLight
  (bind _spotlight_0 (Variables|Default|GetSpotlight_0))
  (Rendering|Components|Light|SetLightColor _spotlight_0 (Variables|Lighting|GetWorriedColor) true)
  (Rendering|Components|Light|SetIntensity _spotlight_0 (Variables|Lighting|GetLight%20Intensity)))

(event Custom|Flickering
  (if (Variables|Lighting|GetIsFlickering)
    (Rendering|Components|Light|SetLightFunctionMaterial (Variables|Default|GetSpotlight_0) "/Game/Blueprints/Lighting_Cole/M_Flickering.M_Flickering")))

(event Custom|Sad%20Light
  (bind _spotlight_0 (Variables|Default|GetSpotlight_0))
  (Rendering|Components|Light|SetLightColor _spotlight_0 (Variables|Lighting|GetSadColor) true)
  (Rendering|Components|Light|SetIntensity _spotlight_0 (Variables|Lighting|GetLight%20Intensity)))

(event EventBeginPlay
  (switch Utilities|FlowControl|Switch|SwitchonEN_CurrentEmotion (Variables|Lighting|GetcurrentEmotion)
    (:NewEnumerator0
      (CallFunction|AnxietyLight)
      (CallFunction|Flickering))
    (:NewEnumerator1
      (CallFunction|SadLight)
      (CallFunction|Flickering))
    (:NewEnumerator2
      (CallFunction|WorriedLight)
      (CallFunction|Flickering))
    (:NewEnumerator3
      (CallFunction|AngerLight)
      (CallFunction|Flickering))))

(fn ConstructionScript)

(fn SadLight)